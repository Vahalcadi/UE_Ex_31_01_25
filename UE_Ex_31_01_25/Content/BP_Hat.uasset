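; BP_Hat is an interactable hat pickup that the player character can collect once.
; On Interact, it passes itself to BP_ThirdPersonCharacter through GiveHat and disables its overlap collision.
; It then notifies GameManagerBP, reached through the game instance, of the pickup, locks out further interaction and removes its interact widget.
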(event EventBeginPlay
  (|CallParentFunction) ; This node is disabled and will not be called.\nDrag off pins to build functionality.
)

(event Collision|EventActorBeginOverlap
  (params (OtherActor :type Actor%20Object%20Reference)))

(event EventTick
  (params (DeltaSeconds :type Float%20%28single-precision%29)))

(fn ConstructionScript
  (|CallParentFunction))

(fn Interact
  (params (Interactor :type Character%20Object%20Reference))
  (if (and (not (Variables|Default|GetisPickedUp?)) (Variables|Default|GetIsInteractable?))
    (bind _asbp_third_person_character (Utilities|Casting|CastToBP_ThirdPersonCharacter Interactor))
    (Default|GiveHat _asbp_third_person_character self)
    (Collision|SetCollisionEnabled (Variables|Default|GetOverlap) "NoCollision")
    (bind _asgame_manager_bp (Utilities|Casting|CastToGameManagerBP (Game|GetGameInstance)))
    (Default|CallOnPickedUpItem _asgame_manager_bp)
    (Variables|Default|SetIsInteractable? false)
    (Variables|Default|SetIsPickedUp? true)
    (Widget|RemovefromParent (Variables|Default|GetInteractWidget))
    (return true)))