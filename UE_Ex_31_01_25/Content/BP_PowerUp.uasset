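; BP_PowerUp is a one-time interactable pickup that changes the interacting third-person character's jump velocity.
; Interact sets the character's JumpZVelocity from the power-up's value, then hides the actor and disables mesh collision instead of destroying it.
; It then notifies GameManagerBP on the Game Instance, sets IsPickedUp to block reuse, and removes the interact widget.
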(event EventBeginPlay
  (|CallParentFunction) ; This node is disabled and will not be called.\nDrag off pins to build functionality.
)

(event Collision|EventActorBeginOverlap
  (params (OtherActor :type Actor%20Object%20Reference)))

(event EventTick
  (params (DeltaSeconds :type Float%20%28single-precision%29)))

(fn ConstructionScript
  (|CallParentFunction))

(fn Interact
  (params (Interactor :type Character%20Object%20Reference))
  (if (not (Variables|Default|GetisPickedUp?))
    (bind _asbp_third_person_character (Utilities|Casting|CastToBP_ThirdPersonCharacter Interactor))
    (Variables|/Script/Engine.CharacterMovementComponent|SetJumpZVelocity (Variables|/Script/Engine.Character|GetCharacterMovement _asbp_third_person_character) (Variables|Default|GetJump%20Z%20Velocity))
    (Development|SetHiddeninGame (Variables|Default|GetDefaultSceneRoot) true true)
    (Collision|SetCollisionEnabled (Variables|Default|GetStaticMesh) "NoCollision")
    (bind _asgame_manager_bp (Utilities|Casting|CastToGameManagerBP (Game|GetGameInstance)))
    (Default|CallOnPickedUpItem _asgame_manager_bp)
    (Variables|Default|SetisPickedUp? true)
    (Widget|RemovefromParent (Variables|Default|GetInteractWidget))
    (return true)))