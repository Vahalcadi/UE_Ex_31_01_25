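; Game manager Blueprint that tracks collected items and decides whether the game can end.
; Init binds AddCount to the item pickup event, incrementing the count and refreshing the HUD's count/max text.
; GenerateViewport creates that HUD, and Reset zeroes the count.
; EndGame shows the game over screen, enables the cursor and pauses when the count equals the maximum, otherwise it prints a message.
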(event Custom|AddCount
  (Variables|Default|SetItemCount (+ (Variables|Default|GetItemCount) 1))
  (CallFunction|UpdateViewport))

(event Custom|EndGame
  (if (== (Variables|Default|GetItemCount) (Variables|Default|GetMaxItemCounter))
    (bind _returnvalue (UserInterface|CreateWidget "/Game/Wid_GameOverScreen.Wid_GameOverScreen_C"))
    (UserInterface|Viewport|AddtoViewport _returnvalue 0)
    (Variables|/Script/Engine.PlayerController|SetbShowMouseCursor (Game|GetPlayerController 0) true)
    (Game|SetGamePaused true)
    (else
      (Development|PrintString "Back to the fields" true true "(R=0.000000,G=0.660000,B=1.000000,A=1.000000)" 5.0))))

(event EventInit
  (EventDispatchers|BindEventtoOnPickedUpItem (delegate Custom|AddCount)))

(fn GenerateViewport
  (bind _returnvalue (UserInterface|CreateWidget "/Game/Wid_HUD.Wid_HUD_C"))
  (bind _output_get (Variables|Default|SetHUD _returnvalue))
  (Rendering|Components|TextRender|SetText (Variables|/Game/Wid_HUD.Wid_HUD_C|GetTextBlock_335 _output_get) (Utilities|Text|ToText(String) (Utilities|String|BuildString(Integer) "" "" (Variables|Default|GetItemCount) (Utilities|String|BuildString(Integer) "" "/" (Variables|Default|GetMaxItemCounter)))))
  (UserInterface|Viewport|AddtoViewport (Variables|Default|GetHUD) 0))

(fn UpdateViewport
  (Rendering|Components|TextRender|SetText (Variables|/Game/Wid_HUD.Wid_HUD_C|GetTextBlock_335 (Variables|Default|GetHUD)) (Utilities|Text|ToText(String) (Utilities|String|BuildString(Integer) "" "" (Variables|Default|GetItemCount) (Utilities|String|BuildString(Integer) "" "/" (Variables|Default|GetMaxItemCounter))))))

(fn Reset
  (Variables|Default|SetItemCount 0)
  (CallFunction|UpdateViewport))