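; BP_PickUp is an interactable pickup that the player collects.
; An overlap component shows an "E" interact prompt widget to the player character while the item is uncollected and removes it when the player leaves.
; Interact hides the item, disables mesh collision, notifies GameManagerBP in the game instance through CallOnPickedUpItem, then sets IsPickedUp and clears the prompt.
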(event OnComponentBeginOverlap(Overlap)
  (params (OverlappedComponent :type Primitive%20Component%20Object%20Reference) (OtherActor :type Actor%20Object%20Reference) (OtherComp :type Primitive%20Component%20Object%20Reference) (OtherBodyIndex :type Integer) (bFromSweep :type Boolean) (SweepResult :type Hit%20Result%20Structure%20%28by%20ref%29))
  (bind _interactwidget (Variables|Default|GetInteractWidget))
  (if (and (== OtherActor (Game|GetPlayerCharacter 0)) (not (Variables|Default|GetisPickedUp?)))
    (Rendering|Components|TextRender|SetText (Variables|/Game/P_Interact.P_Interact_C|GetTextBlock_67 _interactwidget) "Press \"E\" to interact")
    (UserInterface|Viewport|AddtoViewport _interactwidget 0)))

(event OnComponentEndOverlap(Overlap)
  (params (OverlappedComponent :type Primitive%20Component%20Object%20Reference) (OtherActor :type Actor%20Object%20Reference) (OtherComp :type Primitive%20Component%20Object%20Reference) (OtherBodyIndex :type Integer))
  (if (== (Game|GetPlayerCharacter 0) OtherActor)
    (Widget|RemovefromParent (Variables|Default|GetInteractWidget))))

(event EventBeginPlay
  (|CallParentFunction) ; This node is disabled and will not be called.\nDrag off pins to build functionality.
)

(fn ConstructionScript
  (|CallParentFunction))

(fn Interact
  (params (Interactor :type Character%20Object%20Reference))
  (if (not (Variables|Default|GetIsPickedUp?))
    (Development|SetHiddeninGame (Variables|Default|GetDefaultSceneRoot) true true)
    (Collision|SetCollisionEnabled (Variables|Default|GetStaticMesh) "NoCollision")
    (bind _asgame_manager_bp (Utilities|Casting|CastToGameManagerBP (Game|GetGameInstance)))
    (Default|CallOnPickedUpItem _asgame_manager_bp)
    (Variables|Default|SetIsPickedUp? true)
    (Widget|RemovefromParent (Variables|Default|GetInteractWidget))
    (return true)))