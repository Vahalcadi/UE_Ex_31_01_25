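; BP_Key is an interactable key actor that can be picked up once.
; Interact fires the key's OnKeyPickedUp event, hides the actor, disables its mesh collision and notifies GameManagerBP, the game instance, that an item was picked up.
; It then sets the picked-up flag, removes the interact widget and returns true.
; The event graph holds no active logic.
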(event EventBeginPlay
  (|CallParentFunction) ; This node is disabled and will not be called.\nDrag off pins to build functionality.
)

(event Collision|EventActorBeginOverlap
  (params (OtherActor :type Actor%20Object%20Reference)))

(event EventTick
  (params (DeltaSeconds :type Float%20%28single-precision%29)))

(fn ConstructionScript
  (|CallParentFunction))

(fn Interact
  (params (Interactor :type Character%20Object%20Reference))
  (if (not (Variables|Default|GetIsPickedUp?))
    (Default|CallOnKeyPickedUp)
    (Development|SetHiddeninGame (Variables|Default|GetDefaultSceneRoot) true true)
    (Collision|SetCollisionEnabled (Variables|Default|GetStaticMesh) "NoCollision")
    (bind _asgame_manager_bp (Utilities|Casting|CastToGameManagerBP (Game|GetGameInstance)))
    (Default|CallOnPickedUpItem _asgame_manager_bp)
    (Variables|Default|SetIsPickedUp? true)
    (Widget|RemovefromParent (Variables|Default|GetInteractWidget))
    (return true)))